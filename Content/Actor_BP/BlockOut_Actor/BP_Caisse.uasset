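; BP_Caisse is a blockout crate that BP_Humain can push and that counts as shadow cover for BP_Shadow.
; Two trigger volumes, one per X and Y axis, enable physics on the cube and set the human's IsPushing flag on overlap, then clear both on exit.
; A separate Box volume increments the shadow character's IsInShadowCount on entry and decrements it on exit.
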(event `self.Y Axis Collition.OnComponentBeginOverlap`
  (params (OverlappedComponent :type "PrimitiveComponent Object Reference") (OtherActor :type "Actor Object Reference") (OtherComp :type "PrimitiveComponent Object Reference") (OtherBodyIndex :type Integer) (bFromSweep :type Boolean) (SweepResult :type "HitResult Structure (by ref)"))
  ;[0 0 0] Push Y Next in Human BP
  (bind _asbp_humain (cast `/Game/ThirdPerson/Blueprints/Humain_Shadow/BP_Humain` OtherActor))
  (`PrimitiveComponent.SetSimulatePhysics` (`self.Cube`) true)
  (set `/Game/ThirdPerson/Blueprints/Humain_Shadow/BP_Humain.Is Pushing ?` true _asbp_humain))

(event `self.Y Axis Collition.OnComponentEndOverlap`
  (params (OverlappedComponent :type "PrimitiveComponent Object Reference") (OtherActor :type "Actor Object Reference") (OtherComp :type "PrimitiveComponent Object Reference") (OtherBodyIndex :type Integer))
  ;[0 0 0] Push Y Next in Human BP
  (bind _asbp_humain (cast `/Game/ThirdPerson/Blueprints/Humain_Shadow/BP_Humain` OtherActor))
  (`PrimitiveComponent.SetSimulatePhysics` (`self.Cube`) false)
  (set `/Game/ThirdPerson/Blueprints/Humain_Shadow/BP_Humain.Is Pushing ?` false _asbp_humain))

(event `self.X Axis Collition.OnComponentBeginOverlap`
  (params (OverlappedComponent :type "PrimitiveComponent Object Reference") (OtherActor :type "Actor Object Reference") (OtherComp :type "PrimitiveComponent Object Reference") (OtherBodyIndex :type Integer) (bFromSweep :type Boolean) (SweepResult :type "HitResult Structure (by ref)"))
  ;[0 0 0] Push x Next in Human BP
  (bind _asbp_humain (cast `/Game/ThirdPerson/Blueprints/Humain_Shadow/BP_Humain` OtherActor))
  (`PrimitiveComponent.SetSimulatePhysics` (`self.Cube`) true)
  (set `/Game/ThirdPerson/Blueprints/Humain_Shadow/BP_Humain.Is Pushing ?` true _asbp_humain))

(event `self.X Axis Collition.OnComponentEndOverlap`
  (params (OverlappedComponent :type "PrimitiveComponent Object Reference") (OtherActor :type "Actor Object Reference") (OtherComp :type "PrimitiveComponent Object Reference") (OtherBodyIndex :type Integer))
  ;[0 0 0] Push x Next in Human BP
  (bind _asbp_humain (cast `/Game/ThirdPerson/Blueprints/Humain_Shadow/BP_Humain` OtherActor))
  (`PrimitiveComponent.SetSimulatePhysics` (`self.Cube`) false)
  (set `/Game/ThirdPerson/Blueprints/Humain_Shadow/BP_Humain.Is Pushing ?` false _asbp_humain))

(event `self.Box.OnComponentBeginOverlap`
  (params (OverlappedComponent :type "PrimitiveComponent Object Reference") (OtherActor :type "Actor Object Reference") (OtherComp :type "PrimitiveComponent Object Reference") (OtherBodyIndex :type Integer) (bFromSweep :type Boolean) (SweepResult :type "HitResult Structure (by ref)"))
  (bind _asbp_shadow (cast `/Game/ThirdPerson/Blueprints/Humain_Shadow/BP_Shadow` OtherActor))
  (set `/Game/ThirdPerson/Blueprints/Humain_Shadow/BP_Shadow.Is in shadow Count ` (+ (`/Game/ThirdPerson/Blueprints/Humain_Shadow/BP_Shadow.Is in shadow Count ` _asbp_shadow) 1.0) _asbp_shadow))

(event `self.Box.OnComponentEndOverlap`
  (params (OverlappedComponent :type "PrimitiveComponent Object Reference") (OtherActor :type "Actor Object Reference") (OtherComp :type "PrimitiveComponent Object Reference") (OtherBodyIndex :type Integer))
  (bind _asbp_shadow (cast `/Game/ThirdPerson/Blueprints/Humain_Shadow/BP_Shadow` OtherActor))
  (set `/Game/ThirdPerson/Blueprints/Humain_Shadow/BP_Shadow.Is in shadow Count ` (- (`/Game/ThirdPerson/Blueprints/Humain_Shadow/BP_Shadow.Is in shadow Count ` _asbp_shadow) 1.0) _asbp_shadow))

(fn `UserConstructionScript`)