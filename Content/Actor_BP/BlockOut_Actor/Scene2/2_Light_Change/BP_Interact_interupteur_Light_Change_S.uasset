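; Interactable light switch for the Scene 2 light-change blockout that swaps a shadow actor for a spawned light actor.
; On Interact it briefly shows the Off_Light widget, destroys ShadowDestroy and spawns a Mecha_Light_Spawn at the preset location and scale.
; It sets InterupteurShadow and calls Interupteur on all Mecha_Shadow_Change and Mecha_Light_Change actors, with short delays timing the change under the overlay before removing it.
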(event `/Game/Actor_BP/Interact_object/BPI_Interact.Interact`
  (params (Humain :type "/Game/ThirdPerson/Blueprints/Humain_Shadow/BP_Humain Object Reference") (Shadow :type "/Game/ThirdPerson/Blueprints/Humain_Shadow/BP_Shadow Object Reference"))
  (bind _returnvalue (`|CreateWidget` "/Game/Actor_BP/Widget/Off_Light.Off_Light_C"))
  (`UserWidget.AddToViewport` _returnvalue 0)
  (`KismetSystemLibrary.Delay` 0.1)
  (`self.K2_DestroyActor` (`self.Shadow Destroy`))
  (`|SpawnActorFromClass` "/Game/Actor_BP/BlockOut_Actor/Scene2/1_Light_Spawn/Mecha_Light_Spawn.Mecha_Light_Spawn_C" (`KismetMathLibrary.MakeTransform` (`self.Light New Location`) (struct) (`self.Light New Scale`)) "Undefined" "OverrideRootScale" null null)
  (set `self.Interupteur Shadow ?` true)
  (bind _outactors (`GameplayStatics.GetAllActorsOfClass` "/Game/Actor_BP/BlockOut_Actor/Scene2/2_Light_Change/Mecha_Shadow_Change.Mecha_Shadow_Change_C"))
  (`/Game/Actor_BP/BlockOut_Actor/Scene2/2_Light_Change/Mecha_Shadow_Change.interupteur ` _outactors)
  (bind _outactors_2 (`GameplayStatics.GetAllActorsOfClass` "/Game/Actor_BP/BlockOut_Actor/Scene2/2_Light_Change/Mecha_Light_Change.Mecha_Light_Change_C"))
  (`/Game/Actor_BP/BlockOut_Actor/Scene2/2_Light_Change/Mecha_Light_Change.interupteur` _outactors_2)
  (`KismetSystemLibrary.Delay` 0.4)
  (`Widget.RemoveFromParent` _returnvalue))

(fn `UserConstructionScript`)