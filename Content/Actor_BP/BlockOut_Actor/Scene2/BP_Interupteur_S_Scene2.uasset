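; Light switch trigger for Scene 2 that reacts when BP_Shadow overlaps it and swaps the scene's light setup.
; On overlap it briefly shows the Off_Light widget, which covers the change.
; During that window it destroys the referenced ShadowDestroy actor and spawns Mecha_Light_SpawnScene2 using location and scale variables.
; The sequence is timed with short Delays and ends by removing the widget.
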(event `self.ReceiveActorBeginOverlap`
  (params (OtherActor :type "Actor Object Reference"))
  (cast `/Game/ThirdPerson/Blueprints/Humain_Shadow/BP_Shadow` OtherActor)
  (bind _returnvalue (`|CreateWidget` "/Game/Actor_BP/Widget/Off_Light.Off_Light_C"))
  (`UserWidget.AddToViewport` _returnvalue 0)
  (`KismetSystemLibrary.Delay` 0.1)
  (`self.K2_DestroyActor` (`self.Shadow Destroy`))
  (`|SpawnActorFromClass` "/Game/Actor_BP/BlockOut_Actor/Scene2/Mecha_Light_Spawn-Scene2.Mecha_Light_Spawn-Scene2_C" (`KismetMathLibrary.MakeTransform` (`self.Light New Location`) (struct) (`self.Light New Sclae`)) "Undefined" "OverrideRootScale" null null)
  (`KismetSystemLibrary.Delay` 0.4)
  (`Widget.RemoveFromParent` _returnvalue))

(fn `UserConstructionScript`)