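; BP_Interupteur_H_Scene2 is a light switch trigger for Scene 2 that reacts when BP_Humain overlaps it.
; It briefly shows the On_Light1 widget, then destroys the referenced LightDestroy actor and spawns Mecha_Shadow_Spawn_Scene2 at a configured location and scale.
; Short delays sequence the swap behind the widget, which is removed from the viewport afterwards.
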(event `self.ReceiveActorBeginOverlap`
  (params (OtherActor :type "Actor Object Reference"))
  (cast `/Game/ThirdPerson/Blueprints/Humain_Shadow/BP_Humain` OtherActor)
  (bind _returnvalue (`|CreateWidget` "/Game/Actor_BP/Widget/On_Light1.On_Light1_C"))
  (`UserWidget.AddToViewport` _returnvalue 0)
  (`KismetSystemLibrary.Delay` 0.1)
  (`self.K2_DestroyActor` (`self.Light Destroy`))
  (`|SpawnActorFromClass` "/Game/Actor_BP/BlockOut_Actor/Scene2/Mecha_Shadow_Spawn_Scene2.Mecha_Shadow_Spawn_Scene2_C" (`KismetMathLibrary.MakeTransform` (`self.Shadow New Location`) (struct) (`self.Shadow New Scale`)) "Undefined" "OverrideRootScale" null null)
  (`KismetSystemLibrary.Delay` 0.4)
  (`Widget.RemoveFromParent` _returnvalue))

(fn `UserConstructionScript`)