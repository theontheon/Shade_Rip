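; Teleporter trigger for the human character (BP_Humain) in a blockout room, apparently one end of a pair with BP_TP_Human_Salle11.
; Overlapping its capsule calls TP on the human, teleports it to HumainTPLocation, then calls USE on the first BP_TP_Human_Salle11 found by class.
; Its own USE event disables capsule collision for one second, a cooldown that likely prevents an immediate return teleport.
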(event `USE`
  (`PrimitiveComponent.SetCollisionEnabled` (`self.Capsule`) "NoCollision")
  (`KismetSystemLibrary.Delay` 1.0)
  (`PrimitiveComponent.SetCollisionEnabled` (`self.Capsule`) "QueryAndPhysics"))

(event `self.Capsule.OnComponentBeginOverlap`
  (params (OverlappedComponent :type "PrimitiveComponent Object Reference") (OtherActor :type "Actor Object Reference") (OtherComp :type "PrimitiveComponent Object Reference") (OtherBodyIndex :type Integer) (bFromSweep :type Boolean) (SweepResult :type "HitResult Structure (by ref)"))
  (bind _asbp_humain (cast `/Game/ThirdPerson/Blueprints/Humain_Shadow/BP_Humain` OtherActor))
  (`/Game/ThirdPerson/Blueprints/Humain_Shadow/BP_Humain.TP` _asbp_humain)
  (`self.K2_SetActorLocation` _asbp_humain (`self.Humain TP Location `) false true)
  (bind _returnvalue (`GameplayStatics.GetActorOfClass` "/Game/Actor_BP/BlockOut_Actor/SalleGd/BP_TP_Human_Salle-1-1.BP_TP_Human_Salle-1-1_C"))
  (`/Game/Actor_BP/BlockOut_Actor/SalleGd/BP_TP_Human_Salle-1-1.USE` _returnvalue))

(fn `UserConstructionScript`)