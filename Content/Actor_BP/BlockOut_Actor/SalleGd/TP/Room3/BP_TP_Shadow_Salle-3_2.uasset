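; Teleporter trigger for the Shadow character in blockout Room 3.
; When BP_Shadow overlaps the capsule, it calls TP on the Shadow and USE on the BP_TP_Shadow_Salle11 actor, disables its own collision, then moves the Shadow to ShadowTPLocation after a short delay.
; An end overlap from BP_Humain, not the Shadow, re-enables the capsule's collision after a few seconds.
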(event `USE`
  (`PrimitiveComponent.SetCollisionEnabled` (`self.Capsule`) "NoCollision"))

(event `self.Capsule.OnComponentBeginOverlap`
  (params (OverlappedComponent :type "PrimitiveComponent Object Reference") (OtherActor :type "Actor Object Reference") (OtherComp :type "PrimitiveComponent Object Reference") (OtherBodyIndex :type Integer) (bFromSweep :type Boolean) (SweepResult :type "HitResult Structure (by ref)"))
  (bind _asbp_shadow (cast `/Game/ThirdPerson/Blueprints/Humain_Shadow/BP_Shadow` OtherActor))
  (`/Game/ThirdPerson/Blueprints/Humain_Shadow/BP_Shadow.TP` _asbp_shadow)
  (bind _returnvalue (`GameplayStatics.GetActorOfClass` "/Game/Actor_BP/BlockOut_Actor/SalleGd/TP/Room1/BP_TP_Shadow_Salle-1-1.BP_TP_Shadow_Salle-1-1_C"))
  (`/Game/Actor_BP/BlockOut_Actor/SalleGd/TP/Room1/BP_TP_Shadow_Salle-1-1.USE` _returnvalue)
  (`self.USE`)
  (`KismetSystemLibrary.Delay` 0.2)
  (`self.K2_SetActorLocation` _asbp_shadow (`self.Shadow TP Location `) false true))

(event `self.Capsule.OnComponentEndOverlap`
  (params (OverlappedComponent :type "PrimitiveComponent Object Reference") (OtherActor :type "Actor Object Reference") (OtherComp :type "PrimitiveComponent Object Reference") (OtherBodyIndex :type Integer))
  (cast `/Game/ThirdPerson/Blueprints/Humain_Shadow/BP_Humain` OtherActor)
  (`KismetSystemLibrary.Delay` 3.0)
  (`PrimitiveComponent.SetCollisionEnabled` (`self.Capsule`) "QueryAndPhysics"))

(fn `UserConstructionScript`)