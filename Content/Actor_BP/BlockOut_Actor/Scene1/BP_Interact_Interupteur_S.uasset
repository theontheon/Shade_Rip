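; BP_Interact_Interupteur_S is an interactable switch that shifts a scene toward shadow, working opposite BP_Interact_Interupteur_H.
; On Interact, if off, it turns itself on and clears IsOn on the first H switch found via GetActorOfClass.
; A briefly displayed On_Light1 widget covers the change, as Light teleports and rescales to its normal transform and Shadow to its extended one.
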(event `/Game/Actor_BP/Interact_object/BPI_Interact.Interact`
  (params (Humain :type "/Game/ThirdPerson/Blueprints/Humain_Shadow/BP_Humain Object Reference") (Shadow :type "/Game/ThirdPerson/Blueprints/Humain_Shadow/BP_Shadow Object Reference"))
  (if (not (`self.Is On ?`))
    (set `self.Is On ?` true)
    (bind _returnvalue (`GameplayStatics.GetActorOfClass` "/Game/Actor_BP/BlockOut_Actor/Scene1/BP_Interact_Interupteur_H.BP_Interact_Interupteur_H_C"))
    (set `/Game/Actor_BP/BlockOut_Actor/Scene1/BP_Interact_Interupteur_H.Is On ?` false _returnvalue)
    (bind _returnvalue_2 (`|CreateWidget` "/Game/Actor_BP/Widget/On_Light1.On_Light1_C"))
    (`UserWidget.AddToViewport` _returnvalue_2 0)
    (`KismetSystemLibrary.Delay` 0.1)
    ;[0 0 0] Shadow Normal
    (`self.K2_SetActorLocation` (`self.Light`) (`self.Light N Position`) false true)
    (`self.SetActorScale3D` (`self.Light`) (`self.Light N Scale`))
    ;[0 0 0] Light Extend
    (`self.K2_SetActorLocation` (`self.Shadow`) (`self.Shadow E Position`) false true)
    (`self.SetActorScale3D` (`self.Shadow`) (`self.Shadow E Scale`))
    (`KismetSystemLibrary.Delay` 0.4)
    (`Widget.RemoveFromParent` _returnvalue_2)))

(fn `UserConstructionScript`)