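; BP_Interupteur_S is a light switch that reacts when a BP_Shadow actor overlaps it, changing the layout of light and shadow in the scene.
; On overlap it shows an Off_Light widget, then after a brief delay moves and rescales the referenced Light and Shadow actors to preset transforms.
; The widget stays up through the instant change and is removed shortly afterwards.
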(event `self.ReceiveActorBeginOverlap`
  (params (OtherActor :type "Actor Object Reference"))
  (cast `/Game/ThirdPerson/Blueprints/Humain_Shadow/BP_Shadow` OtherActor)
  (bind _returnvalue (`|CreateWidget` "/Game/Actor_BP/Widget/Off_Light.Off_Light_C"))
  (`UserWidget.AddToViewport` _returnvalue 0)
  (`KismetSystemLibrary.Delay` 0.1)
  ;[0 0 0] Light Extend
  (`self.K2_SetActorLocation` (`self.Light`) (`self.Light N Location`) false false)
  (`self.SetActorScale3D` (`self.Light`) (`self.Light N Scale`))
  ;[0 0 0] Shadow Extend
  (`self.K2_SetActorLocation` (`self.Shadow`) (`self.Shadow E Location`) false false)
  (`self.SetActorScale3D` (`self.Shadow`) (`self.Shadow E Scale`))
  (`KismetSystemLibrary.Delay` 0.4)
  (`Widget.RemoveFromParent` _returnvalue))

(fn `UserConstructionScript`)