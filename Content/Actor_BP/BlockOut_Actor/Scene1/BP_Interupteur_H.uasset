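; BP_Interupteur_H is a blockout light switch for Scene1 that triggers when a BP_Humain actor overlaps it.
; On overlap it briefly shows the On_Light1 widget, then teleports the referenced Shadow actor to its normal position and scale and the Light actor to its extended position and scale.
; Short delays time the swap within the widget's display before the widget is removed.
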(event `self.ReceiveActorBeginOverlap`
  (params (OtherActor :type "Actor Object Reference"))
  (cast `/Game/ThirdPerson/Blueprints/Humain_Shadow/BP_Humain` OtherActor)
  (bind _returnvalue (`|CreateWidget` "/Game/Actor_BP/Widget/On_Light1.On_Light1_C"))
  (`UserWidget.AddToViewport` _returnvalue 0)
  (`KismetSystemLibrary.Delay` 0.1)
  ;[0 0 0] Shadow Normal
  (`self.K2_SetActorLocation` (`self.Shadow`) (`self.Shadow N Position `) false false)
  (`self.SetActorScale3D` (`self.Shadow`) (`self.Shadow N Scale`))
  ;[0 0 0] Light Extend
  (`self.K2_SetActorLocation` (`self.Light`) (`self.Light E Position`) false false)
  (`self.SetActorScale3D` (`self.Light`) (`self.Light E Scale`))
  (`KismetSystemLibrary.Delay` 0.4)
  (`Widget.RemoveFromParent` _returnvalue))

(fn `UserConstructionScript`)