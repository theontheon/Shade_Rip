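; Overlap-triggered switch that trades space between a Light actor and a Shadow actor by changing their location and scale.
; IsForHumain selects who can trigger it: BP_Humain extends Light and returns Shadow to normal, while a Shadow character does the reverse.
; Transforms are set instantly from stored variables.
; Used flags on the instance block repeat triggering, and each is cleared only by the opposite branch.
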(event `self.ReceiveActorBeginOverlap`
  (params (OtherActor :type "Actor Object Reference"))
  (if (`self.Is for Humain ? `)
    (cast `/Game/ThirdPerson/Blueprints/Humain_Shadow/BP_Humain` OtherActor)
    (if (not (`self.Humain Is Used`))
      (set `self.Humain Is Used` true)
      (set `self.Shadow Is used` false)
      ;[0 0 0] Shadow Normal
      (`self.K2_SetActorLocation` (`self.Shadow`) (`self.Shadow N Position `) false false)
      (`self.SetActorScale3D` (`self.Shadow`) (`self.Shadow N Scale`))
      ;[0 0 0] Light Extend
      (`self.K2_SetActorLocation` (`self.Light`) (`self.Light E Position`) false false)
      (`self.SetActorScale3D` (`self.Light`) (`self.Light E Scale`)))
    (else
      (cast `/Game/Actor_BP/BlockOut_Actor/Shadow` OtherActor)
      (if (not (`self.Shadow Is used`))
        (set `self.Shadow Is used` true)
        (set `self.Humain Is Used` false)
        ;[0 0 0] Light Extend
        (`self.K2_SetActorLocation` (`self.Light`) (`self.Light N Location`) false false)
        (`self.SetActorScale3D` (`self.Light`) (`self.Light N Scale`))
        ;[0 0 0] Shadow Extend
        (`self.K2_SetActorLocation` (`self.Shadow`) (`self.Shadow E Location`) false false)
        (`self.SetActorScale3D` (`self.Shadow`) (`self.Shadow E Scale`))))))

(fn `UserConstructionScript`)