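; Character component that lets its owner push and pull an object.
; BeginPush attaches the character to the pushable, locks movement-facing rotation and enables Tick; EndPush reverses this.
; Tick remaps externally set move inputs by yaw band, then moves the pushable with a swept, speed-scaled offset, carrying the character along.
; IsPushingObject returns true when no pushable is held, opposite to its name.
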(event `self.ReceiveBeginPlay`
  (`self.SetComponentTickEnabled` false)
  (bind _ascharacter (cast `Character` (`self.GetOwner`)))
  (set `self.Character` _ascharacter))

(event `self.ReceiveTick`
  (params (DeltaSeconds :type "Float (single-precision)"))
  (bind _currentactorzrotation (`self.CurrentActorZRotation`))
  (bind _currentactorzrotation_2 (`self.CurrentActorZRotation`))
  (bind _currentactorzrotation_3 (`self.CurrentActorZRotation`))
  (bind _currentactorzrotation_4 (`self.CurrentActorZRotation`))
  (bind (_returnvalue_roll _returnvalue_pitch _returnvalue_yaw) (`KismetMathLibrary.BreakRotator` (`Actor.K2_GetActorRotation` (`self.Character`))))
  (set `self.CurrentActorZRotation` _returnvalue_yaw)
  ;[1 1 1] Up
  (if (and (>= _currentactorzrotation_2 0.0) (< _currentactorzrotation_2 80.0))
    (bind _currentpushable (`self.CurrentPushable`)
      (:`then`
        (`Actor.K2_AddActorWorldOffset` _currentpushable (`self.GetDeltaLocation` DeltaSeconds (`self.ForwardMove`) (`self.RightMove`)) true false))
      (:`else`))
    (else
      ;[1 1 1] Right
      (if (and (>= _currentactorzrotation_3 80.0) (< _currentactorzrotation_3 170.0))
        (bind _currentpushable_2 (`self.CurrentPushable`)
          (:`then`
            (`Actor.K2_AddActorWorldOffset` _currentpushable_2 (`self.GetDeltaLocation` DeltaSeconds (`self.RightMove`) (* (`self.ForwardMove`) -1.0)) true false))
          (:`else`))
        (else
          ;[1 1 1] Left
          (if (and (>= _currentactorzrotation_4 -90.0) (< _currentactorzrotation_4 0.0))
            (bind _currentpushable_3 (`self.CurrentPushable`)
              (:`then`
                (`Actor.K2_AddActorWorldOffset` _currentpushable_3 (`self.GetDeltaLocation` DeltaSeconds (* (`self.RightMove`) -1.0) (`self.ForwardMove`)) true false))
              (:`else`))
            (else
              ;[1 1 1] Down
              (if (and (>= _currentactorzrotation 180.0) (< _currentactorzrotation 270.0))
                (bind _currentpushable_4 (`self.CurrentPushable`)
                  (:`then`
                    (`Actor.K2_AddActorWorldOffset` _currentpushable_4 (`self.GetDeltaLocation` DeltaSeconds (* (`self.ForwardMove`) -1.0) (* (`self.RightMove`) -1.0)) true false))
                  (:`else`))))))))))

(fn `BeginPush`
  (params (PushableObjectHumain :type "/Game/Actor_BP/PushableObject/Pushable_Object_Humain Object Reference"))
  (locals (OwningCharacter :type "Character Object Reference"))
  (if (not (`KismetSystemLibrary.IsValid` (`self.CurrentPushable`)))
    (bind _ascharacter (cast `Character` (`self.GetOwner`)))
    (set `local.OwningCharacter` _ascharacter)
    (bind _output_get (set `self.CurrentPushable` (`local.PushableObjectHumain`)))
    (`Actor.K2_AttachToActor` (`local.OwningCharacter`) _output_get "None" "KeepWorld" "KeepWorld" "KeepWorld" true)
    (set `CharacterMovementComponent.bOrientRotationToMovement` false (`Character.CharacterMovement` (`local.OwningCharacter`)))
    (`self.SetComponentTickEnabled` true)))

(fn `EndPush`
  (locals (OwningCharacter :type "Character Object Reference"))
  (`self.CurrentPushable`
    (:`then`
      (set `self.CurrentPushable` null)
      (bind _ascharacter (cast `Character` (`self.GetOwner`)))
      (bind _output_get (set `local.OwningCharacter` _ascharacter))
      (`Actor.K2_DetachFromActor` _output_get "KeepWorld" "KeepWorld" "KeepWorld")
      (set `CharacterMovementComponent.bOrientRotationToMovement` true (`Character.CharacterMovement` (`local.OwningCharacter`)))
      (`self.SetComponentTickEnabled` false))
    (:`else`)))

(fn `GetDeltaLocation`
  (params (DeltaSecond :type "Float (double-precision)") (ForwardMove :type "Float (double-precision)") (RightMove :type "Float (double-precision)"))
  (returns (ReturnValue :type "Vector Structure"))
  (set `self.IsMovingObject` (or (!= ForwardMove 0.0) (!= RightMove 0.0)))
  (return (+ (* (* (`Actor.GetActorForwardVector` (`self.Character`)) ForwardMove) (* DeltaSecond (`self.PushSpeed`))) (* (* (`self.PushSpeed`) DeltaSecond) (* RightMove (`Actor.GetActorRightVector` (`self.Character`)))))))

(fn `IsPushingObject`
  (returns (ReturnValue :type Boolean))
  (return (not (`KismetSystemLibrary.IsValid` (`self.CurrentPushable`)))))