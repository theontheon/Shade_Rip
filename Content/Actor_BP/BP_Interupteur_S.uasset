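; BP_Interupteur_S is a switch actor that responds when a BP_Shadow actor begins overlapping it.
; On overlap it moves and rescales the referenced Light actor to its LightN location and scale, and the Shadow actor to its ShadowE location and scale.
; The changes apply instantly without sweeping, and the graph has no end-overlap logic to revert them.
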(event `self.ReceiveActorBeginOverlap`
  (params (OtherActor :type "Actor Object Reference"))
  (cast `/Game/ThirdPerson/Blueprints/Humain_Shadow/BP_Shadow` OtherActor)
  ;[0 0 0] Light Extend
  (`self.K2_SetActorLocation` (`self.Light`) (`self.Light N Location`) false false)
  (`self.SetActorScale3D` (`self.Light`) (`self.Light N Scale`))
  ;[0 0 0] Shadow Extend
  (`self.K2_SetActorLocation` (`self.Shadow`) (`self.Shadow E Location`) false false)
  (`self.SetActorScale3D` (`self.Shadow`) (`self.Shadow E Scale`)))

(fn `UserConstructionScript`)