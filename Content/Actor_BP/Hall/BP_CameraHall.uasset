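; BP_CameraHall is the hall camera actor, tracking the BP_Humain character sideways along the world X axis.
; While Follow is true, Tick looks up BP_Humain each frame and copies its X position, keeping Y and Z fixed.
; The Move event glides a component to a fixed, angled viewpoint and turns following off.
; An unconnected branch that would move back and resume following never runs.
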(event `self.ReceiveBeginPlay`
  (set `self.follow` true))

(event `self.ReceiveTick`
  (params (DeltaSeconds :type "Float (single-precision)"))
  (bind _returnvalue (`GameplayStatics.GetActorOfClass` "/Game/ThirdPerson/Blueprints/Humain_Shadow/BP_Humain.BP_Humain_C"))
  (if (`self.follow`)
    (bind _returnvalue_x (`KismetMathLibrary.BreakVector` (`self.K2_GetActorLocation` _returnvalue)))
    (`self.K2_SetActorLocation` (`KismetMathLibrary.MakeVector` _returnvalue_x 930.0 660.0))))

(event `Move`
  (`KismetSystemLibrary.MoveComponentTo` null (1790.0 1570.0 660.0) (struct :`Pitch` -19.0 :`Yaw` -69.0))
  (set `self.follow` false))

(fn `UserConstructionScript`)